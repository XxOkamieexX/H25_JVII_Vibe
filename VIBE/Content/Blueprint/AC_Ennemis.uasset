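; AC_Ennemis is an enemy component, judging by its name, that tracks a vibe level derived from the player's vibe points.
; Every Tick it casts player 0's character to BP_ThirdPersonCharacter and reads PointDeVibe.
; Two thresholds map that value to a three-tier NiveauDeVibe, which this graph only writes, by polling rather than events.
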(event `self.ReceiveTick`
  (params (DeltaSeconds :type "Float (single-precision)"))
  (bind _asbp_third_person_character (cast `/Game/ThirdPerson/Blueprints/BP_ThirdPersonCharacter` (`GameplayStatics.GetPlayerCharacter` 0)))
  (if (>= (`/Game/ThirdPerson/Blueprints/BP_ThirdPersonCharacter.PointDeVibe` _asbp_third_person_character) 150.0)
    (set `self.NiveauDeVibe` 2)
    (elif (>= (`/Game/ThirdPerson/Blueprints/BP_ThirdPersonCharacter.PointDeVibe` _asbp_third_person_character) 100.0)
      (set `self.NiveauDeVibe` 1)
      (elif (< (`/Game/ThirdPerson/Blueprints/BP_ThirdPersonCharacter.PointDeVibe` _asbp_third_person_character) 100.0)
        (set `self.NiveauDeVibe` 0)))))