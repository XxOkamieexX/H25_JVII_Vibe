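; Poubelle is a trash-bin hazard that drains PointDeVibe from the player's BP_ThirdPersonCharacter when it begins overlapping the Box.
; The amount removed is Degats, which VerifierStadeVibe refreshes every Tick from the NiveauDeVibe level on the ACEnnemis component.
; Levels 0 to 2 map to rising damage through chained equality checks, and any other level leaves Degats unchanged.
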(event `self.Box.OnComponentBeginOverlap`
  (params (OverlappedComponent :type "PrimitiveComponent Object Reference") (OtherActor :type "Actor Object Reference") (OtherComp :type "PrimitiveComponent Object Reference") (OtherBodyIndex :type Integer) (bFromSweep :type Boolean) (SweepResult :type "HitResult Structure (by ref)"))
  (bind _asbp_third_person_character (cast `/Game/ThirdPerson/Blueprints/BP_ThirdPersonCharacter` OtherActor))
  (set `/Game/ThirdPerson/Blueprints/BP_ThirdPersonCharacter.PointDeVibe` (- (`/Game/ThirdPerson/Blueprints/BP_ThirdPersonCharacter.PointDeVibe` _asbp_third_person_character) (`self.Degats`)) _asbp_third_person_character))

(event `self.ReceiveTick`
  (params (DeltaSeconds :type "Float (single-precision)"))
  (`self.VerifierStadeVibe`))

(fn `UserConstructionScript`)

(fn `VerifierStadeVibe`
  (bind _niveaudevibe (`/Game/Blueprint/AC_Ennemis.NiveauDeVibe` (`self.AC_Ennemis`)))
  (if (== _niveaudevibe 0)
    (set `self.Degats` 5.0)
    (return)
    (elif (== _niveaudevibe 1)
      (set `self.Degats` 10.0)
      (return)
      (elif (== _niveaudevibe 2)
        (set `self.Degats` 15.0)
        (return)))))